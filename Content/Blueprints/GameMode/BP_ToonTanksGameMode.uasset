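; BP_ToonTanksGameMode is the Toon Tanks game mode that presents the start and end screens and the match music.
; BeginPlay plays a 2D Megalovania track, and StartGame adds the start-game widget to the viewport.
; GameOver shows a widget with win or loss text from its WonGame flag, then sets Game and UI input and shows the mouse cursor.
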(event `self.ReceiveBeginPlay`
  (`GameplayStatics.PlaySound2D` "/Game/Assets/Audio/y2mate_com_-_Undertale_OST_100__Megalovania.y2mate_com_-_Undertale_OST_100__Megalovania" 1.0 1.0 0.0 null null))

(event `self.StartGame`
  (bind _returnvalue (`|CreateWidget` "/Game/Blueprints/Widgets/WBP_StartGameWidget.WBP_StartGameWidget_C"))
  (`UserWidget.AddToViewport` _returnvalue 0))

(event `self.GameOver`
  (params (bWonGame :type Boolean))
  (bind _returnvalue (`GameplayStatics.GetPlayerController` 0))
  (bind _returnvalue_2 (`|CreateWidget` "/Game/Blueprints/Widgets/WBP_GameOverWidget.WBP_GameOverWidget_C"))
  (`UserWidget.AddToViewport` _returnvalue_2 0)
  (`TextBlock.SetText` (`/Game/Blueprints/Widgets/WBP_GameOverWidget.DisplayText` _returnvalue_2) (select `bool` bWonGame :`false` "You Lost!" :`true` "You Won!" :!type "Text"))
  (`WidgetBlueprintLibrary.SetInputMode_GameAndUIEx` _returnvalue null "DoNotLock" false)
  (set `PlayerController.bShowMouseCursor` true _returnvalue))

(fn `UserConstructionScript`)